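; BP_IA is an AI-driven actor with a simple health and death system.
; On BeginPlay it runs the BT_IA behavior tree and writes the player character's current location, captured only once, to the Destination blackboard key.
; AffectHealth adds a delta to Health, prints the new value, and destroys the actor once Health is zero or below.
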(event EventBeginPlay
  (AI|RunBehaviorTree (AI|GetAIController self) "/Game/IA/BT_IA.BT_IA")
  (AI|Components|Blackboard|SetValueasVector (AI|GetBlackboard self) (Utilities|Name|MakeLiteralName "Destination") (Transformation|GetActorLocation (Game|GetPlayerCharacter 0))))

(event Collision|EventActorBeginOverlap
  (params (OtherActor :type Actor%20Object%20Reference)))

(event EventTick
  (params (DeltaSeconds :type Float%20%28single-precision%29)))

(event EventAffectHealth
  (params (Delta :type Float%20%28single-precision%29))
  (bind _newhealth (CallFunction|UpdateHealthPoint Delta))
  (Development|PrintString (Utilities|String|ToString(Float) _newhealth))
  (if (Variables|Utilities|GetbisDead)
    (Actor|DestroyActor)))

(fn ConstructionScript)

(fn UpdateHealthPoint
  (params (Delta :type Float%20%28single-precision%29))
  (bind _output_get (Variables|Utilities|SetHealth (+ Delta (Variables|Utilities|GetHealth))))
  (CallFunction|UpdateIsDead)
  (return _output_get))

(fn UpdateIsDead
  (if (<= (Variables|Utilities|GetHealth) 0.0)
    (Variables|Utilities|SetbisDead true)
    (else
      (Variables|Utilities|SetbisDead false))))