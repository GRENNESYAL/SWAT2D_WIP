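; BP_ennemy is an enemy character Blueprint that handles taking damage and dying.
; Its AffectHealth event passes a delta to UpdateHealthPoint, prints the result to screen, and destroys the actor when BisDead is set.
; BeginPlay, overlap and Tick are disabled stubs, and the construction script only calls its parent.
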(event EventBeginPlay
  (|CallParentFunction) ; This node is disabled and will not be called.\nDrag off pins to build functionality.
)

(event Collision|EventActorBeginOverlap
  (params (OtherActor :type Actor%20Object%20Reference)))

(event EventTick
  (params (DeltaSeconds :type Float%20%28single-precision%29))
  (|CallParentFunction DeltaSeconds) ; This node is disabled and will not be called.\nDrag off pins to build functionality.
)

(event EventAffectHealth
  (params (Delta :type Float%20%28single-precision%29))
  ;[1 1 1] Gestion damage
  (bind _newhealth (CallFunction|UpdateHealthPoint Delta))
  (Development|PrintString (Utilities|String|ToString(Float) _newhealth))
  (if (Variables|Default|GetbisDead)
    (Actor|DestroyActor)))

(fn ConstructionScript
  (|CallParentFunction))