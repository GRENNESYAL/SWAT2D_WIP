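; Player character for a top-down shooter with flipbook feet animation, cursor-facing aim and a sphere tracking the cursor hit point.
; Movement axes follow control yaw, while sprint and dash change walk speed and share Endurance, drained or regenerated by a timer started on sprint.
; Left click fires the child-actor BP_Pistol and spends ammo, with a delayed refill on R or when empty.
; Health updates set a death flag; DeathGestion is empty.
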(event Custom|BeginPlay%201
  ;[0 1 0] Fix Vitesse de base
  (Variables|/Script/Engine.CharacterMovementComponent|SetMaxWalkSpeed (Variables|Character|GetCharacterMovement) 3e+02))

(event Custom|Tick%203
  (bind _returnvalue (Game|GetPlayerController 0))
  (bind _hitresult (Game|Player|GetHitResultUnderCursorbyChannel _returnvalue "TraceTypeQuery1" true))
  (bind (_bblockinghit _binitialoverlap _time _distance _location _impactpoint _normal _impactnormal) (Collision|BreakHitResult _hitresult))
  (Transformation|SetWorldLocationAndRotation (Variables|Default|GetSphere) _location (Math|Rotator|MakeRotationfromAxes _impactnormal "0, 0, 0" "0, 0, 0") false false))

(event Custom|Tick2
  ;[1 1 0] Animation update
  (CallFunction|UpdateAnimation))

(event Custom|UpdateAnimation
  ;[1 1 0] Handle Animation
  (Sprite|SetFlipbook (Variables|Default|GetFeet) (select (> (Math|Vector|VectorLength (Transformation|GetVelocity)) 0.0) "/Game/Sprite/Player_Character/Animation/Swat_Feet_Animation.Swat_Feet_Animation" "/Game/Sprite/Flipbook/PFB_SWAT_Feet_Idle.PFB_SWAT_Feet_Idle")))

(event Custom|BeginPlay%202
  (Class|ActorComponent|SetIsReplicated (Variables|Default|GetSprite) true))

(event Custom|Tick%201
  ;[0 1 0] Look Mouse
  (Transformation|SetActorRelativeRotation (Math|Rotator|MakeRotator 0.0 0.0 (.Yaw (Math|Rotator|BreakRotator (Math|Rotator|FindLookatRotation (Transformation|GetActorLocation) (.Location (Collision|BreakHitResult (.HitResult (Game|Player|GetHitResultUnderCursorbyChannel (Game|GetPlayerController 0) "TraceTypeQuery1" true))))))))))

(event EventTick
  (params (DeltaSeconds :type Float%20%28single-precision%29))
  ;[1 1 1] Tick Duplicate
  (CallFunction|Tick1)
  (CallFunction|Tick2)
  (CallFunction|Tick3))

(event EventBeginPlay
  ;[1 1 1] Duplicate EventBeginPlay
  (CallFunction|BeginPlay1)
  (CallFunction|BeginPlay2))

(event Input|ActionEvents|InputActionSprint
  (params (Key :type Key%20Structure :default "None"))
  (bind _charactermovement (Variables|Character|GetCharacterMovement))
  ;[0 1 0] Sprint
  (:Pressed
    (if (<= (Variables|Default|GetEndurance) 25.0)
      (Variables|/Script/Engine.CharacterMovementComponent|SetMaxWalkSpeed _charactermovement 3e+02 :!label _label)
      (else
        (Variables|/Script/Engine.CharacterMovementComponent|SetMaxWalkSpeed _charactermovement 6e+02)))
    (bind _returnvalue (Utilities|Time|SetTimerbyFunctionName 0 "GestionStamina" 0.1 true))
    (Variables|Default|SetTimerStamina _returnvalue))
  (:Released
    (goto _label)))

(event Input|ActionEvents|InputActionDash
  (params (Key :type Key%20Structure :default "None"))
  ;[0 1 0] Dash
  (:Pressed
    (if (not (<= (Variables|Default|GetEndurance) 25.0))
      (Variables|/Script/Engine.CharacterMovementComponent|SetMaxWalkSpeed (Variables|Character|GetCharacterMovement) 4e+03)
      (Variables|Default|SetEndurance (- (Variables|Default|GetEndurance) 25.0))
      (Utilities|FlowControl|Delay 0.5)
      (Variables|/Script/Engine.CharacterMovementComponent|SetMaxWalkSpeed (Variables|Character|GetCharacterMovement) 3e+02)
      (Utilities|FlowControl|Delay 0.5))))

(event Input|AxisEvents|InputAxisMovementsLR
  (params (AxisValue :type Float%20%28single-precision%29))
  ;[0 1 0] Movements
  (Pawn|Input|AddMovementInput (Math|Vector|GetForwardVector (Math|Rotator|MakeRotator 0.0 0.0 (.Yaw (Math|Rotator|BreakRotator (Pawn|GetControlRotation :!class /Script/Engine.Pawn))))) AxisValue false))

(event Input|AxisEvents|InputAxisMovementsUD
  (params (AxisValue :type Float%20%28single-precision%29))
  (bind _returnvalue (Pawn|GetControlRotation :!class /Script/Engine.Pawn))
  (bind _yaw (Math|Rotator|BreakRotator _returnvalue))
  (bind _returnvalue_2 (Math|Rotator|MakeRotator 0.0 0.0 _yaw))
  (bind _returnvalue_3 (Math|Vector|GetRightVector _returnvalue_2))
  ;[0 1 0] Movements
  (Pawn|Input|AddMovementInput (- _returnvalue_3 (* _returnvalue_3 2)) AxisValue false))

(event Input|KeyboardEvents|R
  (params (Key :type Key%20Structure :default "None"))
  ;[0 1 0] Pistol
  ;;[0 1 0] Reloading
  (:Pressed
    (if true
      (Variables|Default|SetAmmoPistol (- (Variables|Default|GetAmmoPistol) (Variables|Default|GetAmmoPistol)))
      (Utilities|FlowControl|Delay 1.0)
      (Variables|Default|SetAmmoPistol (+ (Variables|Default|GetAmmoPistol) (Variables|Default|GetMaxAmmoPistol))))))

(event Input|MouseEvents|LeftMouseButton
  (params (Key :type Key%20Structure :default "None"))
  ;[0 1 0] Pistol
  ;;[0 1 0] Tirer
  (:Pressed
    ;;[0 1 0] Reloading
    (if (<= (Variables|Default|GetAmmoPistol) 0.0)
      (Variables|Default|SetAmmoPistol (- (Variables|Default|GetAmmoPistol) (Variables|Default|GetAmmoPistol)))
      (Utilities|FlowControl|Delay 1.0)
      (Variables|Default|SetAmmoPistol (+ (Variables|Default|GetAmmoPistol) (Variables|Default|GetMaxAmmoPistol)))
      (else
        (bind _asbp_pistol (Utilities|Casting|CastToBP_Pistol (Variables|/Script/Engine.ChildActorComponent|GetChildActor (Variables|Default|GetPistol))))
        (Default|Fire _asbp_pistol)
        ;;[0 1 0] Ammo Decrease
        (Variables|Default|SetAmmoPistol (- (Variables|Default|GetAmmoPistol) 1.0))))))

(fn ConstructionScript)

(fn GestionStamina
  (if (Class|MovementComponent|IsExceedingMaxSpeed (Variables|Character|GetCharacterMovement) 3e+02)
    (if (> (Variables|Default|GetEndurance) 0.0)
      ;[1 1 1] Diminution Stamina
      (Variables|Default|SetEndurance (- (Variables|Default|GetEndurance) 2.5))
      (else
        (Variables|/Script/Engine.CharacterMovementComponent|SetMaxWalkSpeed (Variables|Character|GetCharacterMovement) 3e+02)))
    (elif (< (Variables|Default|GetEndurance) (Variables|Default|GetMaxEndurance))
      ;[1 1 1] Regen Stamina
      (Variables|Default|SetEndurance (+ (Variables|Default|GetEndurance) 1.0))
      (else
        (Utilities|Time|PauseTimerbyHandle (Variables|Default|GetTimerStamina))))))

(fn UpdateHealthPoint
  (params (Delta :type Float%20%28single-precision%29))
  ;[1 1 1] Update Health Point
  (bind _output_get (Variables|Default|SetHealth (+ Delta (Variables|Default|GetHealth))))
  (CallFunction|UpdateIsDead)
  (return _output_get))

(fn GestionDash
  (if (Class|MovementComponent|IsExceedingMaxSpeed (Variables|Character|GetCharacterMovement) 3.9e+03)
    (Variables|Default|SetEndurance (+ (Variables|Default|GetEndurance) -25.0))
    (else
      (CallFunction|GestionStamina))))

(fn DeathGestion)

(fn UpdateIsDead
  (if (<= (Variables|Default|GetHealth) 0.0)
    (Variables|Default|SetbisDead true)
    (else
      (Variables|Default|SetbisDead false))))